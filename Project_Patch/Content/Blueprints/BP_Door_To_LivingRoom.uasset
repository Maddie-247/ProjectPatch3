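; Star-gated door that loads the LivingRoom level when the player interacts with it.
; Interact casts the player pawn to BP_ThirdPersonCharacter and requires its Stars to exactly equal StarsNeededToOpen, so a higher count stays locked.
; Debug prints report the locked or unlocked result.
; The EventGraph holds an unconnected copy of the same logic that never runs.
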(fn `Interact`
  (bind _asbp_third_person_character (cast `/Game/ThirdPerson/Blueprints/BP_ThirdPersonCharacter` (`GameplayStatics.GetPlayerCharacter` 0)))
  (if (== (`/Game/ThirdPerson/Blueprints/BP_ThirdPersonCharacter.Stars` _asbp_third_person_character) (`self.Stars Needed To Open`))
    (`KismetSystemLibrary.PrintString` "Unlocked")
    (`GameplayStatics.OpenLevelBySoftObjectPtr` "/Game/Levels/LivingRoom.LivingRoom")
    (`KismetSystemLibrary.PrintString` "Door Opened")
    (else
      (`KismetSystemLibrary.PrintString` "Locked")))
  (return))

(fn `UserConstructionScript`)